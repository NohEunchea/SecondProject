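; BP_Weapon is a weapon actor with a static mesh that reacts to the first-person player's special attack and to contact with survivors.
; Each Tick it casts the player pawn to BP_FirstPersonCharacter and hides the mesh while IsSpecialAttack is set, showing it otherwise.
; Overlapping a BP_Survivor only prints a debug attack message; no damage is applied here.
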(event EventBeginPlay)

(event Collision|EventActorBeginOverlap
  (params (OtherActor :type Actor%20Object%20Reference))
  (Utilities|Casting|CastToBP_Survivor OtherActor)
  (Development|PrintString "ATK SURVIVOR"))

(event EventTick
  (params (DeltaSeconds :type Float%20%28single-precision%29))
  (bind _asbp_first_person_character (Utilities|Casting|CastToBP_FirstPersonCharacter (Game|Player|GetPlayerPawn 0)))
  (if (Variables|/Game/FirstPerson/Blueprints/BP_FirstPersonCharacter.BP_FirstPersonCharacter_C|GetIsSpecialAttack _asbp_first_person_character)
    (Rendering|SetVisibility (Variables|Default|GetStaticMesh) false false)
    (else
      (Rendering|SetVisibility (Variables|Default|GetStaticMesh) true false))))

(fn ConstructionScript)